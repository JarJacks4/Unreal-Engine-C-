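; Main player character Blueprint with a toggleable customization menu and a mobile-only UI.
; BeginPlay creates the mobile widget on Android or iOS and passes a player reference to its meditation button.
; The menu input alternates through a FlipFlop, adding or removing the customization widget while switching cursor, input mode and follow/menu cameras.
; Swap events replace hair, face, torso, legs and feet static meshes, or the body skeletal mesh for race.
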(event `StartMobileUI`
  (bind _returnvalue (`GameplayStatics.GetPlatformName`))
  ; Created The Mobile UI
  ;; If the game is runnin on IOS or android the BP creates the Mobile Widget
  (if (or (== _returnvalue "Android") (`KismetStringLibrary.EqualEqual_StrStr` _returnvalue "IOS"))
    (bind _returnvalue_2 (`|CreateWidget` "/Game/UI/WBP_MobileMenu.WBP_MobileMenu_C"))
    ;; Assigns the android widget to TestMeditationWidget and adds it to the viewport
    (bind _output_get (set `self.TestMeditationWidget` _returnvalue_2))
    (`UserWidget.AddToViewport` _output_get 0)
    ;; Sets a player reference in the UI
    (set `/Game/UI/WBP_Meditation_Button.PlayerRef` self (`/Game/UI/WBP_MobileMenu.WBP_Meditation_Button` _output_get))))

(event `self.ReceiveBeginPlay`
  ; Creates the android widget
  (`self.StartMobileUI`))

(event `EnhancedInput|/Game/Player/Input/Actions/IA_OpenMenu`
  (params (ActionValue :type Boolean) (ElapsedSeconds :type "Float (double-precision)") (TriggeredSeconds :type "Float (double-precision)") (InputAction :type "InputAction Object Reference" :default "/Game/Player/Input/Actions/IA_OpenMenu.IA_OpenMenu"))
  (bind _returnvalue (`GameplayStatics.GetPlayerController` 0))
  ; Opening Customization Window
  (:`Started`
    ;; Doing once so the player does not rapidly open the menu
    (`/Engine/EditorBlueprintResources/StandardMacros.DoOnce` false :!label _label
      (:`Completed`
        (`/Engine/EditorBlueprintResources/StandardMacros.FlipFlop`
          (:`A`
            ;; Adding Customization window to character view and setting it to the game and ui only mode
            (bind _returnvalue_2 (`|CreateWidget` "/Game/UI/WBP_CustomizationMenu.WBP_CustomizationMenu_C" _returnvalue))
            (`UserWidget.AddToViewport` _returnvalue_2 0)
            (set `PlayerController.bShowMouseCursor` true _returnvalue)
            (`WidgetBlueprintLibrary.SetInputMode_GameAndUIEx` _returnvalue _returnvalue_2 "DoNotLock" false)
            (`ActorComponent.SetActive` (`self.MenuCamera`) true false)
            (`ActorComponent.SetActive` (`self.FollowCamera`) false false)
            (`self.ResetMenu`))
          (:`B`
            ;; Removing the Window from character view and setting to Game Mode
            (`Widget.RemoveFromParent` _returnvalue_2)
            (set `PlayerController.bShowMouseCursor` false _returnvalue)
            (`WidgetBlueprintLibrary.SetInputMode_GameOnly` _returnvalue)
            (`ActorComponent.SetActive` (`self.MenuCamera`) false false)
            (`ActorComponent.SetActive` (`self.FollowCamera`) true false)
            (`self.ResetMenu`)))))))

(event `ResetMenu`
  ; Opening Customization Window
  ;; Restting functionality so player can leave the menu
  (goto _label :!via `Reset`))

(event `Swap Hair`
  (params (Hair :type "StaticMesh Object Reference"))
  ; Swap Items on the Main Char
  (`StaticMeshComponent.SetStaticMesh` (`self.Hair`) Hair))

(event `Swap Face`
  (params (Face :type "StaticMesh Object Reference"))
  ; Swap Items on the Main Char
  (`StaticMeshComponent.SetStaticMesh` (`self.Face`) Face))

(event `Swap Torso`
  (params (Torso :type "StaticMesh Object Reference"))
  ; Swap Items on the Main Char
  (`StaticMeshComponent.SetStaticMesh` (`self.Torso`) Torso))

(event `Swap Legs`
  (params (Legs :type "StaticMesh Object Reference"))
  ; Swap Items on the Main Char
  (`StaticMeshComponent.SetStaticMesh` (`self.Legs`) Legs))

(event `Swap Feet`
  (params (Feet :type "StaticMesh Object Reference"))
  ; Swap Items on the Main Char
  (`StaticMeshComponent.SetStaticMesh` (`self.Feet`) Feet))

(event `SwapRace`
  (params (Race :type "SkeletalMesh Object Reference"))
  ; Swap Items on the Main Char
  (`SkeletalMeshComponent.SetSkeletalMeshAsset` (`self.Mesh`) Race))

(fn `UserConstructionScript`)